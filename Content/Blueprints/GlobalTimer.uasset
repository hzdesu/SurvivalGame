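; GlobalTimer runs the day/night cycle and game clock, converting elapsed game time into day, hour and minute with a quarter-day offset.
; Each Tick pitches the sun light from the time of day, updates the sky sphere and recaptures the sky light every frame.
; It tracks a daytime flag from the hour and fires day or night events on changes, which currently only print messages.
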(event `self.ReceiveTick`
  (params (DeltaSeconds :type "Float (single-precision)"))
  (bind _secondsperday (`self.SecondsPerDay`))
  (bind _returnvalue (/ _secondsperday 24.0))
  (bind (_remainder _returnvalue_2) (`KismetMathLibrary.FMod` (+ (`KismetSystemLibrary.GetGameTimeInSeconds`) (/ _secondsperday 4.0)) _secondsperday))
  (bind (_remainder_2 _returnvalue_3) (`KismetMathLibrary.FMod` _remainder _returnvalue))
  (`self.K2_SetActorRotation` (`self.SunLight`) (`KismetMathLibrary.MakeRotator` 0.0 (+ (* (/ _remainder _secondsperday) -360.0) 90.0)) false)
  (`/Engine/EngineSky/BP_Sky_Sphere.UpdateSunDirection` (`self.SkySphere`))
  (`SkyLightComponent.RecaptureSky` (`SkyLight.LightComponent` (`self.SkyLight`)))
  (set `self.CurrentDay` _returnvalue_2)
  (bind _output_get (set `self.CurrentHour` _returnvalue_3))
  (set `self.CurrentMinute` (`.ReturnValue` (`KismetMathLibrary.FMod` _remainder_2 (/ _returnvalue 60.0))))
  (`|ExecutionSequence`
    (:`then_0`
      (if (`self.IsDayTime`)
        (bind _returnvalue_4 (and (<= _output_get 18) (>= _output_get 6)))
        (if (not _returnvalue_4)
          (`self.EnterNightTime`))
        (elif _returnvalue_4
          (`self.EnterDayTime`))))
    (:`then_1`
      (set `self.IsDayTime` _returnvalue_4))))

(event `EnterDayTime`
  (`KismetSystemLibrary.PrintString` "天亮了"))

(event `EnterNightTime`
  (`KismetSystemLibrary.PrintString` "天黑黑"))

(fn `UserConstructionScript`)