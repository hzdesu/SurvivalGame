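; Inventory Blueprint that stores item slots under a weight-based carrying capacity.
; TestCapacity multiplies the item class's default Weight by the count, adds it to the current Load, and reports whether the total fits.
; TryAddItem commits the new Load on success, then either adds the count to a slot of the same type or appends a new slot, returning whether the item was accepted.
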(fn `TestCapacity`
  (params (NewItem :type "/Game/Blueprints/ItemSlot Structure"))
  (returns (Success :type Boolean) (NewLoad :type Integer))
  (bind (_type _name _icon _count) (break `/Game/Blueprints/ItemSlot` NewItem))
  (bind _returnvalue (+ (* (`.Weight` (defaults `Object` _type)) _count) (`self.Load`)))
  (return (<= _returnvalue (`self.Capacity`)) _returnvalue))

(fn `TryAddItem`
  (params (NewItem :type "/Game/Blueprints/ItemSlot Structure"))
  (returns (Success :type Boolean))
  (bind (_type _name _icon _count) (break `/Game/Blueprints/ItemSlot` NewItem))
  (bind (_success _newload) (`self.TestCapacity` NewItem))
  (if _success
    (set `self.Load` _newload)
    (for _array_element (`self.Content`)
      (bind (_type_2 _name_2 _icon_2 _count_2) (break `/Game/Blueprints/ItemSlot` _array_element))
      (if (== _type _type_2)
        (setmembers `/Game/Blueprints/ItemSlot` :`StructRef` _array_element :`Type` _type_2 :`Name` _name_2 :`Icon` _icon_2 :`Count` (+ _count _count_2))
        (return true)))
    (`KismetArrayLibrary.Array_Add` (`self.Content`) NewItem)
    (return true)
    (else
      (return false))))