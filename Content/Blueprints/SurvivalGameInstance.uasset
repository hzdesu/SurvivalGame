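; Survival game instance that shows and hides the runtime UI, pickable panel and inventory panel.
; Each event calls a shared ShowPanel or HidePanel function.
; ShowPanel lazily creates the widget, caches it through a by-ref variable, adds it to the viewport and optionally enables Game-and-UI input with the cursor.
; HidePanel removes the widget and restores game-only input with the cursor hidden.
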(event `CreateRuntimeUI`
  (`self.ShowPanel` null (`self.RuntimeUI`)))

(event `CreatePickablePanel`
  (`self.ShowPanel` "/Game/UI/UI_PickablePanel.UI_PickablePanel_C" (`self.PickablePanel`) true))

(event `HidePickablePanel`
  (`self.HidePanel` (`self.PickablePanel`)))

(event `CreateInventoryPanel`
  (`self.ShowPanel` null (`self.InventoryPanel`) true))

(event `HideInventoryPanel`
  (`self.HidePanel` (`self.InventoryPanel`)))

(fn `HidePanel`
  (params (PanelVar :type "Widget Object Reference"))
  (bind _returnvalue (`GameplayStatics.GetPlayerController` 0))
  (`/Engine/EditorBlueprintResources/StandardMacros.IsValid` PanelVar
    (:`Is Valid`
      (`Widget.RemoveFromParent` PanelVar)
      (`WidgetBlueprintLibrary.SetInputMode_GameOnly` _returnvalue)
      (set `PlayerController.bShowMouseCursor` false _returnvalue))))

(fn `ShowPanel`
  (params (PanelTypeClass :type "UserWidget Class Reference") (PanelVarible :type "UserWidget Object Reference (by ref)") (bChangeUIMode :type Boolean))
  (bind _returnvalue (`GameplayStatics.GetPlayerController` 0))
  (`/Engine/EditorBlueprintResources/StandardMacros.IsValid` PanelVarible
    (:`Is Valid`
      (if (not (`Widget.IsInViewport` PanelVarible))
        (`UserWidget.AddToViewport` PanelVarible 0 :!label _label)
        (if bChangeUIMode
          (`WidgetBlueprintLibrary.SetInputMode_GameAndUIEx` _returnvalue PanelVarible)
          (set `PlayerController.bShowMouseCursor` true _returnvalue))))
    (:`Is Not Valid`
      (bind _returnvalue_2 (`|CreateWidget` PanelTypeClass (`GameplayStatics.GetPlayerController` 0)))
      (`|VariableSetRef` PanelVarible _returnvalue_2)
      (goto _label))))